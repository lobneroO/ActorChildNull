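; BP_Front is a Blueprint actor that tracks the Cube component of a BP_Back child actor held in its Rear component.
; On BeginPlay it casts the Rear child actor to BP_Back and caches its Cube in RearMovedComponent.
; Every Tick it checks that reference for validity and prints whether the rear object exists, using red text when it does not.
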(event `self.ReceiveBeginPlay`
  (`parent.ReceiveBeginPlay`)
  (bind _asbp_back (cast `/Game/BP_Back` (`ChildActorComponent.ChildActor` (`self.Rear`))))
  (set `self.RearMovedComponent` (`/Game/BP_Back.Cube` _asbp_back)))

(event `self.ReceiveTick`
  (params (DeltaSeconds :type "Float (single-precision)"))
  (`parent.ReceiveTick` DeltaSeconds)
  (if (`KismetSystemLibrary.IsValid` (`self.RearMovedComponent`))
    (`KismetSystemLibrary.PrintString` "Rear Object exists")
    (else
      (`KismetSystemLibrary.PrintString` "Rear Object doesn't exist" true true (struct :`R` 1.0 :`A` 1.0)))))

(fn `UserConstructionScript`)